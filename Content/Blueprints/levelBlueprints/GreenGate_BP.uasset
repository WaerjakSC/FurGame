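; Gate Blueprint that raises or lowers its GATE2BODY component when the green lever is pulled.
; Tick polls the GreenLeverPulled flag, and a FlipFlop alternates between moving the body up and down by a fixed world Z offset.
; Each move is a single unswept jump with no interpolation, after which the flag is cleared.
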(event `self.ReceiveTick`
  (params (DeltaSeconds :type "Float (single-precision)"))
  (bind _gate2_body (`self.GATE2_BODY`))
  (bind _returnvalue (`SceneComponent.K2_GetComponentLocation` _gate2_body))
  (if (`self.GreenLeverPulled`)
    (`/Engine/EditorBlueprintResources/StandardMacros.FlipFlop`
      (:`A`
        (`SceneComponent.K2_SetWorldLocation` _gate2_body (+ _returnvalue (0.0 0.0 800.0)) false false)
        (set `self.GreenLeverPulled` false))
      (:`B`
        (`SceneComponent.K2_SetWorldLocation` _gate2_body (+ _returnvalue (0.0 0.0 -800.0)) false false)
        (set `self.GreenLeverPulled` false)))))

(fn `UserConstructionScript`)