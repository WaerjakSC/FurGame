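; Green_Gate_Lever is a lever Blueprint that flags the green gate as pulled when used.
; Use checks InsideDoorTrigger, casts the GreenDoorActor reference to GreenGate_BP, sets its GreenLeverPulled flag and prints a confirmation.
; Begin overlap calls the parent handler, then prints a prompt that the lever can be activated, without filtering the overlapping actor.
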(event `Use`
  (if (`self.InsideDoorTrigger`)
    (bind _asgreen_gate_bp (cast `/Game/Blueprints/levelBlueprints/GreenGate_BP` (`self.GreenDoorActor`)))
    (set `/Game/Blueprints/levelBlueprints/GreenGate_BP.GreenLeverPulled` true _asgreen_gate_bp)
    (`KismetSystemLibrary.PrintString` "You activated the lever!")))

(event `self.ReceiveActorBeginOverlap`
  (params (OtherActor :type "Actor Object Reference"))
  (`parent.ReceiveActorBeginOverlap` OtherActor)
  (`KismetSystemLibrary.PrintString` "You can activate the lever"))

(fn `UserConstructionScript`
  (`parent.UserConstructionScript`))