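; GreenGateBP is a gate actor that opens and closes in response to a green lever.
; Each Tick it checks the GreenLeverPulled flag, which nothing in this Blueprint sets to true.
; When the flag is true, a FlipFlop alternately moves the static mesh up or down by a fixed offset in one instant step, then clears the flag.
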(event `self.ReceiveTick`
  (params (DeltaSeconds :type "Float (single-precision)"))
  (bind _staticmeshcomponent (`self.StaticMeshComponent`))
  (bind _returnvalue (`SceneComponent.K2_GetComponentLocation` _staticmeshcomponent))
  (if (`self.GreenLeverPulled`)
    (`/Engine/EditorBlueprintResources/StandardMacros.FlipFlop`
      (:`A`
        (`SceneComponent.K2_SetWorldLocation` _staticmeshcomponent (+ _returnvalue (0.0 0.0 800.0)) false false)
        (set `self.GreenLeverPulled` false))
      (:`B`
        (`SceneComponent.K2_SetWorldLocation` _staticmeshcomponent (+ _returnvalue (0.0 0.0 -800.0)) false false)
        (set `self.GreenLeverPulled` false)))))

(fn `UserConstructionScript`)