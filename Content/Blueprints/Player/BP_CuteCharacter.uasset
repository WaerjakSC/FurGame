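; Player character Blueprint with Glock and shotgun combat, a kick, lever interaction and a prototype health system.
; Weapons and kick apply point damage through line traces, with the shotgun firing randomly spread pellets that each consume ammo.
; Keys switch guns and trigger delayed reloads from spare ammo.
; BeginPlay creates the HUD and initial stats, while Tick counts down the Glock cooldown and converts collected meat into speed boost values.
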(event `Key|One`
  (params (Key :type "Key Structure"))
  ;[1 1 1] Select Glock
  (:`Pressed`
    (`|ExecutionSequence`
      (:`then_0`
        (set `self.glockSelected_0` true))
      (:`then_1`
        (set `self.gunType` 1)))))

(event `Key|Two`
  (params (Key :type "Key Structure"))
  ;[1 1 1] Select Shotgun
  (:`Pressed`
    (`|ExecutionSequence`
      (:`then_0`
        (set `self.glockSelected_0` false))
      (:`then_1`
        (set `self.gunType` 2)))))

(event `Key|R`
  (params (Key :type "Key Structure"))
  ;[1 1 1] Reloading
  (:`Pressed`
    (set `self.Reloading` true)
    (if (`self.glockSelected_0`)
      (if (`self.haveSpareGlockAmmo`)
        (`KismetSystemLibrary.Delay` 2.0)
        (`|ExecutionSequence`
          (:`then_0`
            (set `self.spareGlockAmmo` (- (`self.spareGlockAmmo`) (- (`self.MaxGlockAmmo`) (`self.GlockAmmo`))))
            (set `self.haveSpareGlockAmmo` (> (`self.spareGlockAmmo`) 0.0)))
          (:`then_1`
            (set `self.GlockAmmo` (`self.MaxGlockAmmo`))))
        (else
          (`KismetSystemLibrary.PrintString` "You do not have enough Ammo to reload!" :!label _label)))
      (elif (`self.haveSpareShotgunAmmo`)
        (`KismetSystemLibrary.Delay` 3.0)
        (`|ExecutionSequence`
          (:`then_0`
            (set `self.spareShotgunAmmo` (- (`self.spareShotgunAmmo`) (- (`self.MaxShotgunAmmo`) (`self.ShotgunAmmo`))))
            (set `self.haveSpareShotgunAmmo` (> (`self.spareShotgunAmmo`) 0.0)))
          (:`then_1`
            (set `self.ShotgunAmmo` (`self.MaxShotgunAmmo`))))
        (else
          (goto _label))))))

(event `Key|LeftMouseButton`
  (params (Key :type "Key Structure"))
  (bind _projectilespawnpoint (`self.ProjectileSpawnPoint`))
  (bind _minimum_spread (`self.Minimum spread`))
  (bind _maximum_spread (`self.Maximum spread`))
  (bind _projectilespawnpoint_2 (`self.ProjectileSpawnPoint`))
  (bind (_returnvalue_roll _returnvalue_pitch _returnvalue_yaw) (`KismetMathLibrary.BreakRotator` (`SceneComponent.K2_GetComponentRotation` _projectilespawnpoint_2)))
  (bind _returnvalue (`SceneComponent.K2_GetComponentLocation` _projectilespawnpoint_2))
  (bind _returnvalue_2 (`SceneComponent.K2_GetComponentLocation` _projectilespawnpoint))
  ;[1 1 1] Character Fires gun
  (:`Pressed`
    (if (`self.Reloading`)
      (`KismetSystemLibrary.PrintString` "Wait until you have finished reloading!")
      (elif (`self.glockSelected_0`)
        ;[1 1 1] Glock
        (if (and (<= (`self.curShotCooldown`) 0.0) (> (`self.GlockAmmo`) 0.0))
          (set `self.curShotCooldown` (`self.shotCooldown`))
          (bind _outhit (`KismetSystemLibrary.LineTraceSingle` :`Start` _returnvalue_2 :`End` (+ _returnvalue_2 (* (`KismetMathLibrary.GetForwardVector` (`SceneComponent.K2_GetComponentRotation` _projectilespawnpoint)) (`self.GunRange`))) :`TraceChannel` "TraceTypeQuery1" :`DrawTime` 1.0))
          (bind (_bblockinghit _binitialoverlap _time _distance _location _impactpoint _normal _impactnormal _physmat _hitactor _hitcomponent _hitbonename _hititem _faceindex _tracestart) (`GameplayStatics.BreakHitResult` _outhit))
          (`GameplayStatics.ApplyPointDamage` _hitactor 100.0 _tracestart _outhit)
          (set `self.GlockAmmo` (- (`self.GlockAmmo`) 1.0))
          (set `self.Shooting` true)
          (else
            (`KismetSystemLibrary.PrintString` "Out of ammo! pres R to reload!" :!label _label_2)))
        (else
          ;[1 1 1] Shotgun
          (if (> (`self.ShotgunAmmo`) 0.0)
            (for _ (range 20)
              (bind _outhit_2 (`KismetSystemLibrary.LineTraceSingle` :`Start` _returnvalue :`End` (+ _returnvalue (* (`KismetMathLibrary.GetForwardVector` (`KismetMathLibrary.MakeRotator` _returnvalue_roll (+ (`KismetMathLibrary.RandomFloatInRange` _minimum_spread _maximum_spread) _returnvalue_pitch) (+ (`KismetMathLibrary.RandomFloatInRange` _minimum_spread _maximum_spread) _returnvalue_yaw))) (`self.ShotgunRange`))) :`TraceChannel` "TraceTypeQuery1" :`DrawDebugType` "ForDuration" :`DrawTime` 1.0))
              (bind (_bblockinghit_2 _binitialoverlap_2 _time_2 _distance_2 _location_2 _impactpoint_2 _normal_2 _impactnormal_2 _physmat_2 _hitactor_2 _hitcomponent_2 _hitbonename_2 _hititem_2 _faceindex_2 _tracestart_2) (`GameplayStatics.BreakHitResult` _outhit_2))
              (`GameplayStatics.ApplyPointDamage` _hitactor_2 20.0 _tracestart_2 _outhit_2)
              (set `self.ShotgunAmmo` (- (`self.ShotgunAmmo`) 1.0)))
            (else
              (goto _label_2))))))))

(event `Key|G`
  (params (Key :type "Key Structure"))
  ;[1 1 1] Test for damage and healing
  (:`Pressed`
    (`self.Health_Deplete`)))

(event `Key|H`
  (params (Key :type "Key Structure"))
  ;[1 1 1] Test for damage and healing
  (:`Pressed`
    (`self.Health_Regen`)))

(event `InputAction|Melee`
  (params (Key :type "Key Structure"))
  (bind _kickarrow (`self.KickArrow`))
  (bind _returnvalue (`SceneComponent.K2_GetComponentLocation` _kickarrow))
  (bind _returnvalue_roll (`KismetMathLibrary.BreakRotator` (`SceneComponent.K2_GetComponentRotation` _kickarrow)))
  ;[1 1 1] Kick attack
  (:`Pressed`
    (bind _outhit (`KismetSystemLibrary.LineTraceSingle` :`Start` _returnvalue :`End` (+ _returnvalue (* (`KismetMathLibrary.GetForwardVector` (`KismetMathLibrary.MakeRotator` _returnvalue_roll)) (`self.KickRange`))) :`TraceChannel` "TraceTypeQuery1" :`DrawDebugType` "ForDuration" :`DrawTime` 1.0))
    (bind (_bblockinghit _binitialoverlap _time _distance _location _impactpoint _normal _impactnormal _physmat _hitactor _hitcomponent _hitbonename _hititem _faceindex _tracestart) (`GameplayStatics.BreakHitResult` _outhit))
    (`GameplayStatics.ApplyPointDamage` _hitactor 50.0 _tracestart _outhit)))

(event `self.ReceiveBeginPlay`
  ;[1 1 1] Create hud and set max and current floats
  (bind _returnvalue (`|CreateWidget` "/Game/Blueprints/Hud_BP.Hud_BP_C" (`GameplayStatics.GetPlayerController` 0)))
  (`UserWidget.AddToViewport` _returnvalue 0)
  (`|ExecutionSequence`
    (:`then_0`
      (set `self.characterHealth` 100.0)
      (set `self.currentCharacterHealth` 100.0))
    (:`then_1`
      (set `self.MaxGlockAmmo` 20.0))
    (:`then_2`
      (set `self.MaxShotgunAmmo` 100.0))))

(event `self.ReceiveTick`
  (params (DeltaSeconds :type "Float (single-precision)"))
  (bind _curshotcooldown (`self.curShotCooldown`))
  ;[1 1 1] In future iterations don't use event tick unless you absolutely have to -- this can be a simple custom event called whenever you pick up more meat
  (if (== (`self.meatCounter`) 10)
    (set `self.meatBoost` (+ (`self.meatBoost`) (`self.10PercentBoost`)))
    (set `self.meatCounter` 0)
    (`KismetSystemLibrary.PrintString` "You got a 10% boost to movement speed!"))
  (if (>= _curshotcooldown 0.0)
    (set `self.curShotCooldown` (- _curshotcooldown DeltaSeconds))))

(event `InputAction|Use`
  (params (Key :type "Key Structure"))
  (:`Pressed`
    (for _array_element (`PrimitiveComponent.GetOverlappingActors` (`self.CapsuleComponent`) "/Game/Blueprints/levelBlueprints/Door_Trigger_Blueprint.Door_Trigger_Blueprint_C")
      (bind _aspink_gate_lever (cast `/Game/Blueprints/levelBlueprints/Pink_Gate_Lever` _array_element))
      (`/Game/Blueprints/levelBlueprints/Pink_Gate_Lever.Use` _aspink_gate_lever))))

(fn `Health_Deplete`
  (bind _output_get (set `self.currentCharacterHealth` (- (`self.currentCharacterHealth`) 20.0)))
  ;[1 1 1] reset health after death just for prototype
  (if (<= _output_get 0.0)
    (set `self.currentCharacterHealth` (`self.characterHealth`))))

(fn `Health_Regen`
  (set `self.currentCharacterHealth` (+ (`self.currentCharacterHealth`) 20.0)))

(fn `UserConstructionScript`)