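; BP_EnemyMelee is a melee enemy Blueprint that hands its behavior to an AI controller.
; On BeginPlay it runs the parent logic, then sets the controller to use MeleeEnemyBlackboard and run the MeleeEnemy behavior tree.
; It adds no other logic of its own: Tick and overlap events are disabled stubs, and the construction script only calls the parent.
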(event `self.ReceiveBeginPlay`
  (bind _returnvalue (`AIBlueprintHelperLibrary.GetAIController` self))
  (`parent.ReceiveBeginPlay`)
  (`AIController.UseBlackboard` _returnvalue "/Game/Blueprints/AI/BehaviorTrees/MeleeEnemyBlackboard.MeleeEnemyBlackboard")
  (`AIController.RunBehaviorTree` _returnvalue "/Game/Blueprints/AI/BehaviorTrees/MeleeEnemy.MeleeEnemy"))

(fn `UserConstructionScript`
  (`parent.UserConstructionScript`))