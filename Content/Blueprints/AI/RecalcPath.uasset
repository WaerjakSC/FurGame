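; Behavior tree task that advances a FurryEnemyPatrol pawn to the next waypoint on its patrol route.
; It writes the waypoint at the CurrentPoint index into the CurrentPatrolPath blackboard key.
; It then increments CurrentPoint, wrapping to zero after the last waypoint so the route loops, and finishes successfully.
; If the pawn is not a FurryEnemyPatrol, the cast fails and the task never calls FinishExecute.
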(event `self.ReceiveExecuteAI`
  (params (OwnerController :type "AIController Object Reference") (ControlledPawn :type "Pawn Object Reference"))
  (bind _returnvalue (`BTFunctionLibrary.GetOwnersBlackboard`))
  (bind _returnvalue_2 (`BlackboardComponent.GetValueAsInt` _returnvalue "CurrentPoint"))
  (bind _asfurry_enemy_patrol (cast `FurryEnemyPatrol` ControlledPawn))
  (bind _waypoints (`FurryEnemyPatrol.Waypoints` _asfurry_enemy_patrol))
  (`BlackboardComponent.SetValueAsObject` _returnvalue (`KismetStringLibrary.Conv_StringToName` "CurrentPatrolPath") (`|GetArrayItem` _waypoints _returnvalue_2))
  (if (== _returnvalue_2 (- (`KismetArrayLibrary.Array_Length` _waypoints) 1))
    (`BlackboardComponent.SetValueAsInt` _returnvalue "CurrentPoint" 0)
    (else
      (`BlackboardComponent.SetValueAsInt` _returnvalue "CurrentPoint" (+ _returnvalue_2 1))))
  (`self.FinishExecute` true))