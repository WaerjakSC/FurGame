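; BP_FurryController is an AI controller that starts waypoint patrol behavior for a BP_FurryEnemyPatrol pawn.
; On BeginPlay it initializes BasicWanderBlackboard, then seeds CurrentPatrolPath with the pawn's first waypoint and CurrentPoint with a zero index.
; It then runs the BasicWander behavior tree, which only starts if the controlled pawn casts to BP_FurryEnemyPatrol.
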(event `self.ReceiveBeginPlay`
  ;[1 1 1] Starts the blackboard and sets blackboard key from the waypoint array.
  (bind _blackboardcomponent (`self.UseBlackboard` "/Game/Blueprints/AI/BehaviorTrees/BasicWanderBlackboard.BasicWanderBlackboard"))
  (bind _asbp_furry_enemy_patrol (cast `/Game/Blueprints/AI/BP_FurryEnemyPatrol` (`self.K2_GetPawn`)))
  (`BlackboardComponent.SetValueAsObject` _blackboardcomponent (`KismetStringLibrary.Conv_StringToName` "CurrentPatrolPath") (`|GetArrayItem` (`FurryEnemyPatrol.Waypoints` _asbp_furry_enemy_patrol)))
  (`BlackboardComponent.SetValueAsInt` _blackboardcomponent "CurrentPoint" 0)
  (`self.RunBehaviorTree` "/Game/Blueprints/AI/BehaviorTrees/BasicWander.BasicWander"))

(fn `UserConstructionScript`)