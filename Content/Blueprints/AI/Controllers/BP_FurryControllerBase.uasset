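; BP_FurryControllerBase is an AI controller base for waypoint-patrolling characters that can react to a nearby player.
; Its startup chain seeds the blackboard with the first waypoint and point index, then runs the BasicWander behavior tree.
; A DoOnce chain sets the Player key and interrupts movement with MoveToLocation.
; Both chains are disconnected and never run, and the PlayerClose event is empty, so the controller currently does nothing.
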(event `PlayerClose`
  ;[1 1 1] Check if player is close and if so set the player in blackboard
)

(fn `UserConstructionScript`)