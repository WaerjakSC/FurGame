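; AI controller for the BP_Baby NPC that drives patrolling and player awareness through a behavior tree.
; On begin play it seeds the blackboard with the pawn's first waypoint entry as the patrol path, then runs the Baby tree.
; Each tick it publishes the pawn's location and checks player distance.
; The first time the player is within range, it stores them in the blackboard and interrupts the current move.
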(event `self.ReceiveBeginPlay`
  ;[1 1 1] Starts the blackboard and sets blackboard key from the waypoint array.
  (bind _blackboardcomponent (`self.UseBlackboard` "/Game/Blueprints/AI/BehaviorTrees/BabyBlackboard.BabyBlackboard"))
  (bind _asbp_baby (cast `/Game/Blueprints/AI/BP_Baby` (`self.K2_GetPawn`)))
  (`BlackboardComponent.SetValueAsObject` _blackboardcomponent (`KismetStringLibrary.Conv_StringToName` "CurrentPatrolPath") (`|GetArrayItem` (`FurryEnemyPatrol.Waypoints` _asbp_baby)))
  (`BlackboardComponent.SetValueAsInt` _blackboardcomponent "CurrentPoint" 0)
  (`self.RunBehaviorTree` "/Game/Blueprints/AI/BehaviorTrees/Baby.Baby"))

(event `PlayerClose`
  (bind _player (`self.Player`))
  (bind _returnvalue (`self.K2_GetActorLocation` (`self.K2_GetPawn`)))
  ;[1 1 1] Check if player is close and if so set the player in blackboard
  (`/Engine/EditorBlueprintResources/StandardMacros.IsValid` _player
    (:`Is Valid`
      _)
    (:`Is Not Valid`
      (bind _outactors (`GameplayStatics.GetAllActorsOfClass` "/Game/Blueprints/Player/BP_MyCuteCharacter.BP_MyCuteCharacter_C"))
      (bind _output_get (set `self.Player` (`|GetArrayItem` _outactors)))))
  (if (<= (`KismetMathLibrary.Vector_Distance` (`self.K2_GetActorLocation` _player) _returnvalue) 1500.0)
    (`/Engine/EditorBlueprintResources/StandardMacros.DoOnce` false
      (:`Completed`
        (`BlackboardComponent.SetValueAsObject` (`AIBlueprintHelperLibrary.GetBlackboard` null) "Player" _output_get)
        (`BlackboardComponent.SetValueAsObject` (`AIBlueprintHelperLibrary.GetBlackboard` null) "Player" _output_get)
        ;;[1 1 1] Interrupts any current moveTo orders
        (`self.MoveToLocation` _returnvalue -1.0 true true false true null)))))

(event `self.ReceiveTick`
  (params (DeltaSeconds :type "Float (single-precision)"))
  (bind _returnvalue (`AIBlueprintHelperLibrary.GetBlackboard` null))
  ;[1 1 1] Make the NPC face the player when aware of it
  (`self.PlayerClose`)
  (`BlackboardComponent.SetValueAsVector` _returnvalue "SelfLocation" (`self.K2_GetActorLocation` (`self.K2_GetPawn`)))
  (`/Engine/EditorBlueprintResources/StandardMacros.IsValid` (`BlackboardComponent.GetValueAsObject` _returnvalue "Player")))

(fn `UserConstructionScript`)