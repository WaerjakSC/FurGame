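; Shotgun choke pickup that tightens the player's pellet spread by pulling the maximum and minimum spread values inward by a fixed step.
; A looping timeline continuously yaws the Cylinder mesh from its initial rotation.
; Any overlap destroys the pickup before the cast to BP_MyCuteCharacter, which then receives the spread change.
; Debug prints show the results, though the minimum's print adds the step a second time.
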(event `self.ReceiveBeginPlay`
  (bind (_initil_rotation_cylinder_roll _initil_rotation_cylinder_pitch _initil_rotation_cylinder_yaw) (`KismetMathLibrary.BreakRotator` (`self.Initil Rotation Cylinder`)))
  (set `self.Initil Rotation Cylinder` (`SceneComponent.K2_GetComponentRotation` (`self.Cylinder`)))
  (bind (_direction _newtrack_0) (`Timeline|Timeline_0` :!label _label)
    (:`Update`
      (`SceneComponent.K2_SetWorldRotation` (`self.Cylinder`) (`KismetMathLibrary.MakeRotator` _initil_rotation_cylinder_roll _initil_rotation_cylinder_pitch (+ _newtrack_0 _initil_rotation_cylinder_yaw)) false false))
    (:`Finished`
      (goto _label :!via `PlayFromStart`))))

(event `self.ReceiveActorBeginOverlap`
  (params (OtherActor :type "Actor Object Reference"))
  (`self.K2_DestroyActor`)
  (bind _asbp_my_cute_character (cast `/Game/Blueprints/Player/BP_MyCuteCharacter` OtherActor))
  (`|ExecutionSequence`
    (:`then_0`
      (bind _maximum_spread (`/Game/Blueprints/Player/BP_MyCuteCharacter.Maximum spread` _asbp_my_cute_character))
      (set `/Game/Blueprints/Player/BP_MyCuteCharacter.Maximum spread` (- _maximum_spread 2.5) _asbp_my_cute_character)
      (`KismetSystemLibrary.PrintString` (`KismetStringLibrary.Conv_DoubleToString` _maximum_spread)))
    (:`then_1`
      (bind _returnvalue (+ (`/Game/Blueprints/Player/BP_MyCuteCharacter.Minimum spread` _asbp_my_cute_character) 2.5))
      (set `/Game/Blueprints/Player/BP_MyCuteCharacter.Minimum spread` _returnvalue _asbp_my_cute_character)
      (`KismetSystemLibrary.PrintString` (`KismetStringLibrary.Conv_DoubleToString` _returnvalue)))))

(fn `UserConstructionScript`)