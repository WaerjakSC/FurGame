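; Meat pickup that spins in the level and feeds the BP_CuteCharacter that touches it.
; A looping timeline adds yaw to the Cube's starting rotation.
; Any actor overlap destroys the pickup before the cast, so non-character actors also consume it.
; For the character, it increments both meat counters and adds a fifth of CharacterHealth to current health, with no clamp here.
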(event `self.ReceiveBeginPlay`
  (bind (_initialrotation_roll _initialrotation_pitch _initialrotation_yaw) (`KismetMathLibrary.BreakRotator` (`self.InitialRotation`)))
  (set `self.InitialRotation` (`SceneComponent.K2_GetComponentRotation` (`self.Cube`)))
  (bind (_direction _newtrack_0) (`Timeline|Timeline_0` :!label _label)
    (:`Update`
      (`SceneComponent.K2_SetWorldRotation` (`self.Cube`) (`KismetMathLibrary.MakeRotator` _initialrotation_roll _initialrotation_pitch (+ _newtrack_0 _initialrotation_yaw)) false false))
    (:`Finished`
      (goto _label :!via `PlayFromStart`))))

(event `self.ReceiveActorBeginOverlap`
  (params (OtherActor :type "Actor Object Reference"))
  (`self.K2_DestroyActor`)
  (bind _asbp_cute_character (cast `/Game/Blueprints/Player/BP_CuteCharacter` OtherActor))
  (`|ExecutionSequence`
    (:`then_0`
      (set `/Game/Blueprints/Player/BP_CuteCharacter.meatEaten` (+ (`/Game/Blueprints/Player/BP_CuteCharacter.meatEaten` _asbp_cute_character) 1) _asbp_cute_character))
    (:`then_1`
      (set `/Game/Blueprints/Player/BP_CuteCharacter.meatCounter` (+ (`/Game/Blueprints/Player/BP_CuteCharacter.meatCounter` _asbp_cute_character) 1) _asbp_cute_character))
    (:`then_2`
      (set `CuteCharacter.currentCharacterHealth` (+ (`CuteCharacter.currentCharacterHealth` _asbp_cute_character) (/ (`CuteCharacter.characterHealth` _asbp_cute_character) 5.0)) _asbp_cute_character))))

(fn `UserConstructionScript`)