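; Glock ammo upgrade pickup that raises the player character's maximum Glock ammo by a fixed amount.
; A looping timeline spins the AmmoUpgrade component in yaw, offset from its initial rotation.
; On overlap it destroys itself before casting to BP_CuteCharacter, so any overlapping actor consumes it, but only that character receives the MaxGlockAmmo increase.
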(event `self.ReceiveBeginPlay`
  (bind (_initialrotation_roll _initialrotation_pitch _initialrotation_yaw) (`KismetMathLibrary.BreakRotator` (`self.initialRotation`)))
  (set `self.initialRotation` (`SceneComponent.K2_GetComponentRotation` (`self.Ammo upgrade`)))
  (bind (_direction _newtrack_0) (`Timeline|Timeline_0` :!label _label)
    (:`Update`
      (`SceneComponent.K2_SetWorldRotation` (`self.Ammo upgrade`) (`KismetMathLibrary.MakeRotator` _initialrotation_roll _initialrotation_pitch (+ _newtrack_0 _initialrotation_yaw)) false false))
    (:`Finished`
      (goto _label :!via `PlayFromStart`))))

(event `self.ReceiveActorBeginOverlap`
  (params (OtherActor :type "Actor Object Reference"))
  (`self.K2_DestroyActor`)
  (bind _asbp_cute_character (cast `/Game/Blueprints/Player/BP_CuteCharacter` OtherActor))
  (set `/Game/Blueprints/Player/BP_CuteCharacter.MaxGlockAmmo` (+ (`/Game/Blueprints/Player/BP_CuteCharacter.MaxGlockAmmo` _asbp_cute_character) 50.0) _asbp_cute_character))

(fn `UserConstructionScript`)