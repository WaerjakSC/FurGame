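; Key pickup actor that spins in place and gives the player character a key on overlap.
; A looping timeline started on BeginPlay adds a yaw offset to the cube's initial rotation.
; Any overlap destroys the actor first, then sets HasKey if the other actor casts to BP_MyCuteCharacter, so non-player overlaps also remove the key.
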(event `self.ReceiveBeginPlay`
  (bind (_initial_rotation_roll _initial_rotation_pitch _initial_rotation_yaw) (`KismetMathLibrary.BreakRotator` (`self.Initial Rotation`)))
  (set `self.Initial Rotation` (`SceneComponent.K2_GetComponentRotation` (`self.Cube`)))
  (bind (_direction _newtrack_0) (`Timeline|Timeline_0` :!label _label)
    (:`Update`
      (`SceneComponent.K2_SetWorldRotation` (`self.Cube`) (`KismetMathLibrary.MakeRotator` _initial_rotation_roll _initial_rotation_pitch (+ _newtrack_0 _initial_rotation_yaw)) false false))
    (:`Finished`
      (goto _label :!via `PlayFromStart`))))

(event `self.ReceiveActorBeginOverlap`
  (params (OtherActor :type "Actor Object Reference"))
  (`self.K2_DestroyActor`)
  (bind _asbp_my_cute_character (cast `/Game/Blueprints/Player/BP_MyCuteCharacter` OtherActor))
  (set `/Game/Blueprints/Player/BP_MyCuteCharacter.hasKey` true _asbp_my_cute_character))

(fn `UserConstructionScript`)